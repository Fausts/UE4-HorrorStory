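; Player controller for the zombie world mode, shared by the horror master and hero roles, handling match-state UI and commander drag movement.
; Notify events show the settlement screen or, for heroes only, a game-over screen, and respawn rebinds the hero in-game HUD.
; LeftTouch drag records start positions and moves the pawn through a gate, scaling mouse delta with a 60-degree cosine correction.
; Tick is an empty stub; cursor look-at rotation is unused.
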(event `NotifySettlement`
  (params (IsMasterWin :type Boolean))
  (`WidgetLayoutLibrary.RemoveAllWidgets`)
  (bind _returnvalue (`|CreateWidget` "/Game/HorrorStory/ZombieWorldScene/Blueprints/UI/UI_Settlement.UI_Settlement_C" self IsMasterWin))
  (`UserWidget.AddToViewport` _returnvalue 0))

(event `NotifyHeroDown`
  (if (not (`self.IsHorrorMaster`))
    (bind _returnvalue (`|CreateWidget` "/Game/HorrorStory/ZombieWorldScene/Blueprints/UI/UI_HeroGameOver.UI_HeroGameOver_C" self))
    (`UserWidget.AddToViewport` _returnvalue 0)))

(event `self.OC_OnRespawnPlayer`
  (bind _asui_hero_in_game (cast `/Game/HorrorStory/ZombieWorldScene/Blueprints/UI/UI_HeroInGame` (`self.InGameHUDRef`)))
  (`/Game/HorrorStory/ZombieWorldScene/Blueprints/UI/UI_HeroInGame.SetupEventBind` _asui_hero_in_game))

(event `InputAction|LeftTouch` :consume false
  (params (Key :type "Key Structure" :default "AnyKey"))
  (bind (_locationx _locationy) (`self.GetMousePosition`))
  (bind (_locationx_2 _locationy_2) (`self.GetMousePosition`))
  (bind (_returnvalue_x _returnvalue_y) (`KismetMathLibrary.BreakVector` (- (`self.TouchStartMousePosition`) (`KismetMathLibrary.MakeVector` _locationx_2 _locationy_2))))
  ;[1 1 1] Record mouse and commander position when touch start
  (:`Pressed`
    (set `self.TouchStartMousePosition` (`KismetMathLibrary.MakeVector` _locationx _locationy))
    (set `self.TouchStartCommanderPosition` (`self.K2_GetActorLocation` (`self.K2_GetPawn`)))
    (`/Engine/EditorBlueprintResources/StandardMacros.Gate` true :!via `Open` :!label _label ; While key is pressed...
      (:`Exit`
        (`self.K2_SetActorLocation` (`self.K2_GetPawn`) (+ (`self.TouchStartCommanderPosition`) (* (* (`KismetMathLibrary.MakeVector` _returnvalue_y (* _returnvalue_x -1.0 (`KismetMathLibrary.DegCos` 60.0))) -1.0) (`self.MouseMoveScale`))) false false))))
  (:`Released`
    (goto _label :!via `Close`)))

(event `self.ReceiveTick`
  (params (DeltaSeconds :type "Float (single-precision)"))
  (`/Engine/EditorBlueprintResources/StandardMacros.IsValid` (`self.K2_GetPawn`)
    (:`Is Valid`
      (if (`self.IsHorrorMaster`)
        _))))

(fn `UserConstructionScript`)