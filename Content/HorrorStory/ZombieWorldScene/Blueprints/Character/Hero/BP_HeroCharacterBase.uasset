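; Base hero character for a networked top-down zombie shooter, with movement, weapon firing and slot switching, health, shield and speed-up.
; Tick aims the character via a cursor hit interpolated toward the camera to eye height, and traces the laser beam.
; Fire, shield and death replicate through multicasts; WeaponComponent spawns bullets on the server when animation triggers them.
; Death ragdolls the mesh and notifies the local controller; Health replication updates the bar.
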(event `self.ReceiveBeginPlay`
  (`|ExecutionSequence`
    (:`then_0`
      ;[1 1 1] add myself into ai storage
      (bind _outactors (`GameplayStatics.GetAllActorsOfClass` "/Game/AIBehaviorToolkit/Blueprints/BP_AIStorage.BP_AIStorage_C"))
      (if (> (`KismetArrayLibrary.Array_Length` _outactors) 0)
        (`/Game/AIBehaviorToolkit/Blueprints/BP_AIStorage.AddActorToList` (`KismetArrayLibrary.Array_Get` _outactors) self)))
    (:`then_1`
      ;[1 1 1] gun  laser
      (bind _returnvalue (`GameplayStatics.SpawnEmitterAtLocation` "/Game/HorrorStory/Common/Blueprints/TricksAndTraps/RotatingLaserTransmitter/P_Laser.P_Laser" (0.0 0.0 0.0) (struct) false))
      (bind _output_get (set `self.P_GunLaser` _returnvalue))
      (`SceneComponent.SetHiddenInGame` _output_get true false))
    (:`then_2`
      (`KismetSystemLibrary.Delay` 0.5) ; wait a little time for possess compelete
      (if (`self.IsLocallyControlled`)
        ;[1 1 1] spawn fog of war
        (`|ExecutionSequence`
          (:`then_1`
            ;[1 1 1] spawn gun aim target
            (bind _returnvalue_2 (`|SpawnActorFromClass` "/Game/HorrorStory/ZombieWorldScene/Blueprints/Character/Hero/GunAimTarget/BP_GunAimTarget.BP_GunAimTarget_C" (`KismetMathLibrary.MakeTransform` (0.0 0.0 0.0)) "Undefined" "OverrideRootScale"))
            (set `self.GunAimTarget` _returnvalue_2)))))))

(event `self.ReceiveTick`
  (params (DeltaSeconds :type "Float (single-precision)"))
  (bind _bulletspawnarrow (`self.BulletSpawnArrow`))
  (bind _p_gunlaser (`self.P_GunLaser`))
  (bind _returnvalue (`SceneComponent.K2_GetComponentLocation` _bulletspawnarrow))
  (bind _returnvalue_2 (`PlayerCameraManager.GetCameraLocation` (`GameplayStatics.GetPlayerCameraManager` 0)))
  (`|ExecutionSequence`
    (:`then_0`
      ;[1 1 1] set gun aim target
      (`self.GunAimTarget`
        (:`then`
          (bind _asplayer_controller (cast `PlayerController` (`self.GetController`)))
          (bind (_bblockinghit _binitialoverlap _time _location) (`GameplayStatics.BreakHitResult` (`PlayerController.GetHitResultUnderCursorForObjects` _asplayer_controller (`|MakeArray` "ObjectTypeQuery7" :!type "EObjectTypeQuery Enum") true)))
          (bind _returnvalue_3 (`KismetMathLibrary.VLerp` _location _returnvalue_2 (/ (+ (`CapsuleComponent.GetScaledCapsuleHalfHeight` (`self.CapsuleComponent`)) (`self.BaseEyeHeight`)) (- (.z _returnvalue_2) (.z _location)))))
          (bind _returnvalue_4 (`KismetMathLibrary.FindLookAtRotation` (`self.GetActorEyesViewPoint`) _returnvalue_3))
          (`self.K2_SetActorLocationAndRotation` (`self.GunAimTarget`) _returnvalue_3 _returnvalue_4 false false)
          (`Controller.SetControlRotation` _asplayer_controller _returnvalue_4) ; set controller rotation
        )
        (:`else`)))
    (:`then_1`
      ;[1 1 1] set laser
      (bind _outhit (`KismetSystemLibrary.LineTraceSingleForObjects` _returnvalue (+ _returnvalue (* (`SceneComponent.GetForwardVector` _bulletspawnarrow) 5000.0)) (`|MakeArray` "ObjectTypeQuery1" :!type "EObjectTypeQuery Enum")))
      (bind (_bblockinghit_2 _binitialoverlap_2 _time_2 _location_2 _impactpoint _normal _impactnormal _physmat _hitactor _hitcomponent _hitbonename _hititem _faceindex _tracestart _traceend) (`GameplayStatics.BreakHitResult` _outhit))
      (`ParticleSystemComponent.SetBeamSourcePoint` (`self.P_GunLaser`) 0 _tracestart 0)
      (if _bblockinghit_2
        (`ParticleSystemComponent.SetBeamTargetPoint` _p_gunlaser 0 _location_2 0)
        (else
          (`ParticleSystemComponent.SetBeamTargetPoint` _p_gunlaser 0 _traceend 0))))))

(event `OpenShield`
  ;[1 1 1] Item
  ;;[1 1 1] Shield
  (`self.MC_OpenShield`)
  (`Timeline|TimelineShield` :!via `PlayFromStart`
    (:`Finished`
      (`self.MC_CloseShield`))))

(event `self.ReceiveAnyDamage`
  (params (Damage :type "Float (single-precision)") (DamageType :type "DamageType Object Reference") (InstigatedBy :type "Controller Object Reference") (DamageCauser :type "Actor Object Reference"))
  ;[1 1 1] damage and death
  ;;[1 1 1] Reduce Health based on damage
  (if (not (`self.IsImmortal`))
    (bind _output_get (set `self.Health` (- (`self.Health`) Damage)))
    (if (<= _output_get 0.0)
      (`/Engine/EditorBlueprintResources/StandardMacros.DoOnce` false
        (:`Completed`
          (`self.MC_OnDeath`))))))

(event `MC_OpenShield`
  ;[1 1 1] Item
  ;;[1 1 1] Shield
  (set `self.IsImmortal` true)
  (`SceneComponent.SetHiddenInGame` (`self.ShieldMesh`) false false))

(event `MC_CloseShield`
  ;[1 1 1] Item
  ;;[1 1 1] Shield
  (set `self.IsImmortal` false)
  (`SceneComponent.SetHiddenInGame` (`self.ShieldMesh`) true false))

(event `Speedup`
  ;[1 1 1] Item
  ;;[1 1 1] speed up
  (set `CharacterMovementComponent.MaxWalkSpeed` 1200.0 (`self.CharacterMovement`))
  (`Timeline|TimelineSpeedup` :!via `PlayFromStart`
    (:`Finished`
      (set `CharacterMovementComponent.MaxWalkSpeed` 600.0 (`self.CharacterMovement`)))))

(event `MC_OnDeath`
  (bind _returnvalue (`self.GetController`))
  (bind _capsulecomponent (`self.CapsuleComponent`))
  (bind _mesh (`self.Mesh`))
  ;[1 1 1] damage and death
  (`|ExecutionSequence`
    (:`then_0`
      ;;[1 1 1] Default ragdoll death event
      (`PrimitiveComponent.SetCollisionResponseToAllChannels` _capsulecomponent "ECR_Ignore")
      (`PrimitiveComponent.SetCollisionResponseToChannel` _capsulecomponent "ECC_WorldStatic" "ECR_Block")
      (`PrimitiveComponent.SetCollisionProfileName` _mesh "Ragdoll")
      (`PrimitiveComponent.SetSimulatePhysics` _mesh true)
      (`AnimInstance.Montage_Stop` (`SkeletalMeshComponent.GetAnimInstance` _mesh) 0.0 null)
      ;;[1 1 1] clear tags
      (set `self.Tags` (`|MakeArray` "None" :!type "Name")))
    (:`then_1`
      ;;[1 1 1] disable owning client input and show game over widget
      (if (`KismetSystemLibrary.IsValid` _returnvalue)
        (if (`Controller.IsLocalPlayerController` _returnvalue)
          (`/Game/HorrorStory/ZombieWorldScene/Blueprints/GameModeEtc/BP_ZombieWorldPlayerController.NotifyHeroDown` (cast `/Game/HorrorStory/ZombieWorldScene/Blueprints/GameModeEtc/BP_ZombieWorldPlayerController` _returnvalue :!pure true)))))))

(event `ModifyHP`
  (params (ChangeHP :type "Float (double-precision)"))
  ;[1 1 1] Item
  ;;[1 1 1] ModifyHP
  (`/Engine/EditorBlueprintResources/ActorMacros.Switch Has Authority`
    (:`Authority`
      (set `self.Health` (`KismetMathLibrary.FClamp` (+ (`self.Health`) ChangeHP) 0.0 (`self.MaxHealth`))))))

(event `SpawnBullet`
  (bind _bulletspawnarrow (`self.BulletSpawnArrow`))
  ;[1 1 1] bullet spawn, invoked by animation instance
  (`/Engine/EditorBlueprintResources/ActorMacros.Switch Has Authority`
    (:`Authority`
      (`/Game/HorrorStory/ZombieWorldScene/Blueprints/Character/Hero/Weapon/WeaponComponent.Server_SpawnBullet` (`self.WeaponComponent`) (`SceneComponent.K2_GetComponentRotation` _bulletspawnarrow) (`SceneComponent.K2_GetComponentLocation` _bulletspawnarrow)))))

(event `self.ReceiveDestroyed`
  (`|ExecutionSequence`
    (:`then_0`
      (`self.FogOfWar`
        (:`then`
          (`self.K2_DestroyActor`))
        (:`else`)))
    (:`then_1`
      (bind _gunaimtarget (`self.GunAimTarget`)
        (:`then`
          (`self.K2_DestroyActor` _gunaimtarget))
        (:`else`)))))

(event `InputAxis|MoveForward`
  (params (AxisValue :type "Float (single-precision)"))
  ;[1 1 1] Movement
  (`self.AddMovementInput` (1.0 0.0 0.0) AxisValue))

(event `InputAxis|MoveRight`
  (params (AxisValue :type "Float (single-precision)"))
  ;[1 1 1] Movement
  (`self.AddMovementInput` (0.0 1.0 0.0) AxisValue))

(event `InputAction|Fire`
  (params (Key :type "Key Structure" :default "AnyKey"))
  ;[1 1 1] Fire
  (:`Pressed`
    (`self.Server_OnFire` true))
  (:`Released`
    (`self.Server_OnFire` false)))

(event `Server_OnFire`
  (params (IsAttacking :type Boolean))
  ;[1 1 1] Fire
  (`self.MC_OnFire` IsAttacking))

(event `MC_OnFire`
  (params (IsAttacking :type Boolean))
  (bind _returnvalue (not IsAttacking))
  ;[1 1 1] Fire
  (`/Game/HorrorStory/ZombieWorldScene/Blueprints/Character/Hero/Weapon/WeaponComponent.SetIsAttacking` (`self.WeaponComponent`) IsAttacking)
  (set `CharacterMovementComponent.bOrientRotationToMovement` _returnvalue (`self.CharacterMovement`))
  (set `self.bUseControllerRotationYaw` IsAttacking)
  (`SceneComponent.SetHiddenInGame` (`self.P_GunLaser`) _returnvalue false))

(event `InputAction|EquipLastWeapon`
  (params (Key :type "Key Structure" :default "AnyKey"))
  ;[1 1 1] Equip weapon
  (:`Pressed`
    (`self.Server_EquipLastSlotWeapon`)))

(event `InputAction|EquipNextWeapon`
  (params (Key :type "Key Structure" :default "AnyKey"))
  ;[1 1 1] Equip weapon
  (:`Pressed`
    (`self.Server_EquipNextSlotWeapon`)))

(event `Server_EquipLastSlotWeapon`
  ;[1 1 1] Equip weapon
  (`/Game/HorrorStory/ZombieWorldScene/Blueprints/Character/Hero/Weapon/WeaponComponent.MC_SwitchWeaponSlot` (`self.WeaponComponent`) (cast `/Game/HorrorStory/ZombieWorldScene/Blueprints/Character/Hero/Weapon/Enum_WeaponSlotType` (- (`/Game/HorrorStory/ZombieWorldScene/Blueprints/Character/Hero/Weapon/WeaponComponent.GetCurrentActivingSlot` (`self.WeaponComponent`)) 1))))

(event `Server_EquipNextSlotWeapon`
  ;[1 1 1] Equip weapon
  (`/Game/HorrorStory/ZombieWorldScene/Blueprints/Character/Hero/Weapon/WeaponComponent.MC_SwitchWeaponSlot` (`self.WeaponComponent`) (cast `/Game/HorrorStory/ZombieWorldScene/Blueprints/Character/Hero/Weapon/Enum_WeaponSlotType` (+ (`/Game/HorrorStory/ZombieWorldScene/Blueprints/Character/Hero/Weapon/WeaponComponent.GetCurrentActivingSlot` (`self.WeaponComponent`)) 1))))

(fn `OnRep_Health`
  (`self.Update A Bar` "Health" (/ (`self.Health`) (`self.MaxHealth`))))

(fn `UserConstructionScript`)